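; Fireplace puzzle actor that is put out when an actor tagged "water" overlaps its trigger box.
; The overlap deactivates the fire, destroys the trigger and the water actor, and plays the extinguish effect.
; It also flags SpotLight_Blueprint actors tagged "FireplaceLight" to dim.
; Tick fades its own point light toward zero with a delta-time lerp until intensity reads exactly zero.
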(event OnComponentBeginOverlap(BoxTrigger)
  (params (OverlappedComponent :type Primitive%20Component%20Object%20Reference) (OtherActor :type Actor%20Object%20Reference) (OtherComp :type Primitive%20Component%20Object%20Reference) (OtherBodyIndex :type Integer) (bFromSweep :type Boolean) (SweepResult :type Hit%20Result%20Structure%20%28by%20ref%29))
  (if (Actor|ActorHasTag OtherActor "water")
    (Components|Activation|Deactivate (Variables|Default|GetFire))
    (Components|DestroyComponent (Variables|Default|GetBoxTrigger))
    (Actor|DestroyActor OtherActor)
    (Audio|Components|Audio|Play (Variables|Default|GetExtinguish) 1.0)
    (Variables|Default|SetbDimLight true)
    (bind _outactors (Actor|GetAllActorswithTag "FireplaceLight"))
    (for _array_element _outactors
      (bind _asspot_light_blueprint (Utilities|Casting|CastToSpotLight_Blueprint _array_element))
      (Variables|/Game/Lighting/SpotLight_Blueprint.SpotLight_Blueprint_C|SetbShouldDim _asspot_light_blueprint true))))

(event Custom|DimLight
  (bind _pointlight (Variables|Default|GetPointLight))
  (bind _intensity (Variables|/Script/Engine.LightComponentBase|GetIntensity _pointlight))
  (Rendering|Components|Light|SetIntensity _pointlight (Math|Float|Lerp _intensity 0.0 (* (Utilities|Time|GetWorldDeltaSeconds) 2.0)))
  (if (== _intensity 0.0)
    (Variables|Default|SetbDimLight false)))

(event EventBeginPlay)

(event Collision|EventActorBeginOverlap
  (params (OtherActor :type Actor%20Object%20Reference)))

(event EventTick
  (params (DeltaSeconds :type Float%20%28single-precision%29))
  (if (Variables|Default|GetbDimLight)
    (CallFunction|DimLight)))

(fn ConstructionScript)