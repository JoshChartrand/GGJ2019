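; Light switch puzzle actor that turns off its light the first time its player overlap event fires.
; The event plays Switch, destroys the Light component and flags the SpotLight to dim.
; Tick then calls DimLight, which lerps intensity toward zero using frame delta time.
; Once intensity nears a low threshold, short of zero, dimming stops and PuzzleComplete plays.
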(event EventBeginPlay
  (|CallParentFunction) ; This node is disabled and will not be called.\nDrag off pins to build functionality.
)

(event Collision|EventActorBeginOverlap
  (params (OtherActor :type Actor%20Object%20Reference))
  (|CallParentFunction OtherActor) ; This node is disabled and will not be called.\nDrag off pins to build functionality.
)

(event EventTick
  (params (DeltaSeconds :type Float%20%28single-precision%29))
  (|CallParentFunction DeltaSeconds)
  (if (Variables|Default|GetbShouldDim)
    (CallFunction|DimLight)))

(event EventPlayerOverlapEvent
  (Utilities|FlowControl|DoOnce false
    (:Completed
      (Variables|Default|SetbShouldDim true)
      (Audio|Components|Audio|Play (Variables|Default|GetSwitch) 0.0)
      (Components|DestroyComponent (Variables|Default|GetLight)))))

(fn ConstructionScript
  (|CallParentFunction))

(fn DimLight
  (bind _spotlight (Variables|Default|GetSpotLight))
  (bind _intensity (Variables|/Script/Engine.LightComponentBase|GetIntensity _spotlight))
  (Rendering|Components|Light|SetIntensity _spotlight (Math|Float|Lerp _intensity 0.0 (* (Utilities|Time|GetWorldDeltaSeconds) 5.0)))
  (if (Math|Float|NearlyEqual(Float) _intensity 25.0 5.0)
    (Variables|Default|SetbShouldDim false)
    (Audio|Components|Audio|Play (Variables|Default|GetPuzzleComplete) 0.0)))